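; BP_ObstaclePipe is an obstacle made of two pipe meshes separated vertically by a configurable gap, with a randomized height.
; The construction script scales both meshes and derives offsets from half their height, assuming a 100-unit base, plus half the gap.
; RandomizePosition shifts both by one random Z, placing StaticMeshDown at the positive offset and StaticMeshUp at the negative.
; The event graph has no active logic.
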(fn `RandomizePosition`
  (locals (RandomZ :type "Float (double-precision)" :default 0.0))
  (set `local.RandomZ` (`KismetMathLibrary.RandomFloatInRange` (`self.MinZ`) (`self.MaxZ`)))
  (`SceneComponent.K2_SetRelativeLocation` (`self.StaticMeshDown`) (`KismetMathLibrary.MakeVector` 0.0 0.0 (+ (`self.PipeUpPosition`) (`local.RandomZ`))) false false)
  (`SceneComponent.K2_SetRelativeLocation` (`self.StaticMeshUp`) (`KismetMathLibrary.MakeVector` 0.0 0.0 (+ (`self.PipeDownPosition`) (`local.RandomZ`))) false false))

(fn `UserConstructionScript`
  (bind _pipescale (`self.PipeScale`))
  (bind (_pipescale_x _pipescale_y _pipescale_z) (`KismetMathLibrary.BreakVector` (`self.PipeScale`)))
  (bind _returnvalue (+ (/ (* _pipescale_z 100.0) 2.0) (/ (`self.Gap`) 2.0)))
  (`SceneComponent.SetRelativeScale3D` (`self.StaticMeshUp`) _pipescale)
  (`SceneComponent.SetRelativeScale3D` (`self.StaticMeshDown`) _pipescale)
  (set `self.PipeUpPosition` _returnvalue)
  (set `self.PipeDownPosition` (* _returnvalue -1.0))
  (`self.RandomizePosition`))