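; Level manager for a Flippy Birb game that controls the main menu, game start, game over and the shared level speed.
; BeginPlay zeroes the speed and shows the main menu, handing itself to both menu widgets.
; StartGame enables pawn gravity and uses a timeline to ramp up to the speed cached at construction; GameOver stops it and shows its menu.
; A Bounds volume notifies each overlapping obstacle's owning spawner.
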(event `self.ReceiveBeginPlay`
  (bind _returnvalue (`GameplayStatics.GetPlayerController` 0))
  (bind _outactors (`GameplayStatics.GetAllActorsOfClass` "/Game/Blueprints/BP_FlippyBirbPawn.BP_FlippyBirbPawn_C"))
  (set `self.PlayerPawn` (`|GetArrayItem` _outactors))
  (set `self.LevelSpeed` 0.0)
  (bind _returnvalue_2 (`|CreateWidget` "/Game/UI/WBP_GameOverMenu.WBP_GameOverMenu_C"))
  (set `self.GameOverMenu` _returnvalue_2)
  (set `/Game/UI/WBP_GameOverMenu.LevelManager` self (`self.GameOverMenu`))
  (bind _returnvalue_3 (`|CreateWidget` "/Game/UI/WBP_MainMenu.WBP_MainMenu_C"))
  (set `/Game/UI/WBP_MainMenu.LevelManager` self _returnvalue_3)
  (`UserWidget.AddToViewport` _returnvalue_3 0)
  (`WidgetBlueprintLibrary.SetInputMode_UIOnlyEx` _returnvalue null)
  (set `PlayerController.bShowMouseCursor` true _returnvalue))

(event `self.Bounds.OnComponentBeginOverlap`
  (params (OverlappedComponent :type "PrimitiveComponent Object Reference") (OtherActor :type "Actor Object Reference") (OtherComp :type "PrimitiveComponent Object Reference") (OtherBodyIndex :type Integer) (bFromSweep :type Boolean) (SweepResult :type "HitResult Structure (by ref)"))
  (bind _asbp_obstacle_base (cast `/Game/Blueprints/Obstacles/BP_ObstacleBase` OtherActor))
  (bind _asspawner_base (cast `SpawnerBase` (`self.GetOwner` _asbp_obstacle_base)))
  (`SpawnerBase.SpawnedActorHitBounds` _asspawner_base _asbp_obstacle_base))

(event `self.GameOver`
  (bind _returnvalue (`GameplayStatics.GetPlayerController` 0))
  (if (not (`self.bIsGameOver`))
    (set `self.bIsGameOver` true)
    (set `self.LevelSpeed` 0.0)
    (`UserWidget.AddToViewport` (`self.GameOverMenu`) 0)
    (`WidgetBlueprintLibrary.SetInputMode_UIOnlyEx` _returnvalue null)
    (set `PlayerController.bShowMouseCursor` true _returnvalue)))

(event `self.StartGame`
  (bind _returnvalue (`GameplayStatics.GetPlayerController` 0))
  (`PrimitiveComponent.SetEnableGravity` (`/Game/Blueprints/BP_FlippyBirbPawn.StaticMesh` (`self.PlayerPawn`)) true)
  (bind (_direction _speedalpha) (`Timeline|StartingGame`)
    (:`Update`
      (set `self.LevelSpeed` (`KismetMathLibrary.Lerp` 0.0 (`self.DefaultSpeed`) _speedalpha))
      (set `self.bIsGameOver` false)
      (`WidgetBlueprintLibrary.SetInputMode_GameOnly` _returnvalue)
      (set `PlayerController.bShowMouseCursor` false _returnvalue))))

(fn `UserConstructionScript`
  (`SceneComponent.K2_SetRelativeLocation` (`self.Bounds`) (`self.BoundsLocation`) false false)
  (set `self.DefaultSpeed` (`self.LevelSpeed`)))