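; BP_SpawnerFloor is a child spawner Blueprint for floor obstacles that sets its spacing from the floor's size.
; Its construction script instantiates the spawn class, casts it to BP_ObstacleFloor, and converts FloorScale.X to an X-only DistanceBetweenActors at 100 units per scale.
; When a spawned actor hits the bounds, it defers the parent's handling with a zero-second Delay.
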(event `self.ReceiveBeginPlay`
  (`parent.ReceiveBeginPlay`))

(event `self.SpawnedActorHitBounds`
  (params (Actor :type "Actor Object Reference"))
  (`KismetSystemLibrary.Delay` 0.0)
  (`parent.SpawnedActorHitBounds` Actor))

(fn `UserConstructionScript`
  (`parent.UserConstructionScript`)
  (bind _returnvalue (`|GenericCreateObject` (`self.ActorClassToBeSpawned`)))
  (bind _asbp_obstacle_floor (cast `/Game/Blueprints/Obstacles/BP_ObstacleFloor` _returnvalue))
  (bind _floorscale_x (`KismetMathLibrary.BreakVector` (`/Game/Blueprints/Obstacles/BP_ObstacleFloor.FloorScale` _asbp_obstacle_floor)))
  (set `self.DistanceBetweenActors` (`KismetMathLibrary.MakeVector` (* _floorscale_x 100.0))))