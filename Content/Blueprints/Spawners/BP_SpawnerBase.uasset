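; BP_SpawnerBase is a base spawner that handles what happens when one of its spawned actors hits the bounds.
; With Repeat set, that actor is destroyed; otherwise it is recycled to DistanceBetweenActors past LastSpawnedActor and becomes the new last actor.
; A separate Init event caches the first BP_LevelManager in the level.
; BeginPlay is empty, and no spawning logic lives in this graph.
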(event `self.ReceiveBeginPlay`)

(event `self.SpawnedActorHitBounds`
  (params (Actor :type "Actor Object Reference"))
  (if (`self.bRepeat`)
    (`self.K2_DestroyActor` Actor)
    (else
      (`self.K2_SetActorLocation` Actor (+ (`self.K2_GetActorLocation` (`self.LastSpawnedActor`)) (`self.DistanceBetweenActors`)) false false)
      (set `self.LastSpawnedActor` Actor))))

(event `self.Init`
  (bind _outactors (`GameplayStatics.GetAllActorsOfClass` "/Game/Blueprints/BP_LevelManager.BP_LevelManager_C"))
  (set `self.LevelManager` (`|GetArrayItem` _outactors)))

(fn `UserConstructionScript`)