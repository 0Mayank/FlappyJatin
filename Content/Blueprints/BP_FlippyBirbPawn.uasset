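; BP_FlippyBirbPawn is the bird pawn for a Flappy Bird-style game, handling collision-triggered game over.
; It turns off mesh gravity on BeginPlay; no movement logic lives in this graph.
; Hitting a BP_ObstacleBase reaches the LevelManager through the obstacle's owning SpawnerBase and calls GameOver.
; Any hit also adds IMC_GameOver at priority 1 for a player controller, while the IMC_Default removal node is unconnected.
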(event `self.ReceiveBeginPlay`
  (`PrimitiveComponent.SetEnableGravity` (`self.StaticMesh`) false))

(event `self.StaticMesh.OnComponentHit`
  (params (HitComponent :type "PrimitiveComponent Object Reference") (OtherActor :type "Actor Object Reference") (OtherComp :type "PrimitiveComponent Object Reference") (NormalImpulse :type "Vector Structure") (Hit :type "HitResult Structure (by ref)"))
  (`|ExecutionSequence`
    (:`then_0`
      (bind _asbp_obstacle_base (cast `/Game/Blueprints/Obstacles/BP_ObstacleBase` OtherActor))
      (bind _asspawner_base (cast `SpawnerBase` (`self.GetOwner` _asbp_obstacle_base)))
      (`LevelManager.GameOver` (`SpawnerBase.GetLevelManager` _asspawner_base)))
    (:`then_1`
      (bind _asplayer_controller (cast `PlayerController` (`self.GetController`)))
      (`EnhancedInputSubsystemInterface.AddMappingContext` (pcsubsystem `EnhancedInputLocalPlayerSubsystem` _asplayer_controller) "/Game/Input/IMC_GameOver.IMC_GameOver" 1 (struct)))))

(fn `UserConstructionScript`)